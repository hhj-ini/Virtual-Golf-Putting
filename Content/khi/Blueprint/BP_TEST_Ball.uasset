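; BP_TEST_Ball is a test ball actor that the player pushes around with the arrow keys.
; On BeginPlay it enables input from player controller 0.
; Each arrow key press applies a one-shot physics impulse to the Sphere component along the world X or Y axis, scaled by a Power variable.
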(event `self.ReceiveBeginPlay`
  (`self.EnableInput` (`GameplayStatics.GetPlayerController` 0)))

(event `Key|Up`
  (params (Key :type "Key Structure"))
  (:`Pressed`
    (`PrimitiveComponent.AddImpulse` (`self.Sphere`) (* (1.0 0.0 0.0) (`self.Power`)) "None" false)))

(event `Key|Down`
  (params (Key :type "Key Structure"))
  (:`Pressed`
    (`PrimitiveComponent.AddImpulse` (`self.Sphere`) (* (* (1.0 0.0 0.0) (`self.Power`)) -1.0) "None" false)))

(event `Key|Right`
  (params (Key :type "Key Structure"))
  (:`Pressed`
    (`PrimitiveComponent.AddImpulse` (`self.Sphere`) (* (0.0 1.0 0.0) (`self.Power`)) "None" false)))

(event `Key|Left`
  (params (Key :type "Key Structure"))
  (:`Pressed`
    (`PrimitiveComponent.AddImpulse` (`self.Sphere`) (* (* (0.0 1.0 0.0) (`self.Power`)) -1.0) "None" false)))

(fn `UserConstructionScript`)