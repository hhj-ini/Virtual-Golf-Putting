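; Actor component that keeps its owner's static mesh on "green" ground, resetting it when it strays onto another surface.
; BeginPlay caches the mesh and its starting location and enables overlap events.
; Each Tick traces straight down from the mesh and checks the hit physical material's surface type.
; A hit on any surface other than SurfaceType1 teleports the mesh back to start and clears its physics velocities.
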(event `self.ReceiveBeginPlay`
  (bind _output_get (set `self.static mesh` (`Actor.GetComponentByClass` (`self.GetOwner`) "/Script/Engine.StaticMeshComponent")))
  (set `self.Start Location` (`SceneComponent.K2_GetComponentLocation` _output_get))
  (set `PrimitiveComponent.bGenerateOverlapEvents` true _output_get))

(event `self.ReceiveTick`
  (params (DeltaSeconds :type "Float (single-precision)"))
  (bind _static_mesh (`self.static mesh`))
  (bind _returnvalue (`SceneComponent.K2_GetComponentLocation` (`self.static mesh`)))
  (bind (_outhit _returnvalue_2) (`KismetSystemLibrary.LineTraceSingle` _returnvalue (+ _returnvalue (0.0 0.0 -10000.0)) "TraceTypeQuery4"))
  (if _returnvalue_2
    (if (not (`|EnumEquality` (`PhysicalMaterial.SurfaceType` (`.PhysMat` (`GameplayStatics.BreakHitResult` _outhit))) "SurfaceType1"))
      (`SceneComponent.K2_SetWorldLocation` _static_mesh (`self.Start Location`) false false)
      (`PrimitiveComponent.SetAllPhysicsLinearVelocity` _static_mesh (0.0 0.0 0.0) false)
      (`PrimitiveComponent.SetAllPhysicsAngularVelocityInRadians` _static_mesh (0.0 0.0 0.0) false))))