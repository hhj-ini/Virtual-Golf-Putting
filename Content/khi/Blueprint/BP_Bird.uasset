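; BP_Bird is a bird actor that plays a chirp sound repeatedly.
; A looping one-second timer started on BeginPlay calls Chirp, which plays ChirpSound only while the Chrip flag is clear.
; Chirp sets the flag, and the sound's OnAudioFinished event clears it, so playback never restarts mid-chirp.
; A random 50% check exists but is unused, so chirps are not randomized.
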(event `self.ReceiveBeginPlay`
  (add `AudioComponent.OnAudioFinished` (`self.ChirpSound`) (delegate `OnAudioFinished_Event`))
  (`KismetSystemLibrary.K2_SetTimerDelegate` (delegate `CustomEvent`) 1.0 true))

(event `CustomEvent`
  (`self.Chirp`))

(event `OnAudioFinished_Event`
  (set `self.Chrip?` false))

(fn `Chirp`
  (if (and (not (`self.Chrip?`)) true)
    (`AudioComponent.Play` (`self.ChirpSound`) 0.0)
    (set `self.Chrip?` true)))

(fn `UserConstructionScript`)