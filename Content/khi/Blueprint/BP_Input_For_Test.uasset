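; Debug input actor that maps keyboard keys to test actions in the game.
; On BeginPlay it enables input for the first player and caches the GM_Base_UI game mode and the bird manager.
; Number keys trigger a height-change call, bird relocation around the player, golf ball spawning on the VR character and black ball destruction.
; Arrow keys and Z apply forces to the black ball's sphere, looking it up on each press.
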(event `self.ReceiveBeginPlay`
  (`self.EnableInput` (`GameplayStatics.GetPlayerController` 0))
  (bind _asgm_base_ui (cast `/Game/ljh/Bluerprint/GM_Base_UI` (`GameplayStatics.GetGameMode`)))
  (set `self.GM` _asgm_base_ui)
  (bind _returnvalue (`GameplayStatics.GetActorOfClass` "/Game/khi/Blueprint/BP_BirdManager.BP_BirdManager_C"))
  (set `self.Bird Manager` _returnvalue))

(event `Key|One`
  (params (Key :type "Key Structure"))
  (:`Pressed`
    (`/Game/ljh/Bluerprint/GM_Base_UI.ChangedHeightInteger` (`self.GM`))))

(event `Key|Two`
  (params (Key :type "Key Structure"))
  (:`Pressed`
    (`/Game/khi/Blueprint/BP_BirdManager.RelocateBirdsAroundPlayer` (`self.Bird Manager`))))

(event `Key|Three`
  (params (Key :type "Key Structure"))
  (:`Pressed`
    (bind _returnvalue (`GameplayStatics.GetActorOfClass` "/Game/hhz/class/BP_VRCharacter_UI_Child.BP_VRCharacter_UI_Child_C"))
    (`/Engine/EditorBlueprintResources/StandardMacros.IsValid` _returnvalue
      (:`Is Valid`
        (`/Game/hhz/class/BP_VRCharacter_UI_Child.SpawnGolfBall` _returnvalue))
      (:`Is Not Valid`
        (`KismetSystemLibrary.PrintString` "not")))))

(event `Key|Four`
  (params (Key :type "Key Structure"))
  (:`Pressed`
    (bind _returnvalue (`GameplayStatics.GetActorOfClass` "/Game/hhz/class/BP_BalckBall.BP_BalckBall_C"))
    (`self.K2_DestroyActor` _returnvalue)))

(event `Key|Right`
  (params (Key :type "Key Structure"))
  (:`Pressed`
    (bind _returnvalue (`GameplayStatics.GetActorOfClass` "/Game/hhz/class/BP_BalckBall.BP_BalckBall_C"))
    (`PrimitiveComponent.AddForce` (`/Game/hhz/class/BP_BalckBall.Sphere` _returnvalue) (0.0 100.0 0.0) "None" false)))

(event `Key|Up`
  (params (Key :type "Key Structure"))
  (:`Pressed`
    (bind _returnvalue (`GameplayStatics.GetActorOfClass` "/Game/hhz/class/BP_BalckBall.BP_BalckBall_C"))
    (`PrimitiveComponent.AddForce` (`/Game/hhz/class/BP_BalckBall.Sphere` _returnvalue) (100.0 100.0 0.0) "None" false)))

(event `Key|Left`
  (params (Key :type "Key Structure"))
  (:`Pressed`
    (bind _returnvalue (`GameplayStatics.GetActorOfClass` "/Game/hhz/class/BP_BalckBall.BP_BalckBall_C"))
    (`PrimitiveComponent.AddForce` (`/Game/hhz/class/BP_BalckBall.Sphere` _returnvalue) (0.0 -100.0 0.0) "None" false)))

(event `Key|Down`
  (params (Key :type "Key Structure"))
  (:`Pressed`
    (bind _returnvalue (`GameplayStatics.GetActorOfClass` "/Game/hhz/class/BP_BalckBall.BP_BalckBall_C"))
    (`PrimitiveComponent.AddForce` (`/Game/hhz/class/BP_BalckBall.Sphere` _returnvalue) (-100.0 0.0 0.0) "None" false)))

(event `Key|Z`
  (params (Key :type "Key Structure"))
  (:`Pressed`
    (bind _returnvalue (`GameplayStatics.GetActorOfClass` "/Game/hhz/class/BP_BalckBall.BP_BalckBall_C"))
    (`PrimitiveComponent.AddForce` (`/Game/hhz/class/BP_BalckBall.Sphere` _returnvalue) (0.0 0.0 -10000.0) "None" false)))

(fn `UserConstructionScript`)