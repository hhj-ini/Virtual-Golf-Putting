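; BP_BirdManager spawns and tracks a flock of BP_Bird actors and plays forest ambient sound.
; On BeginPlay it starts the 2D sound, then spawns NumOfBird birds at its own transform and stores them in the Birds array.
; RelocateBirdsAroundPlayer moves each bird to a GetRandomDest location and writes a separately requested random destination to its Blackboard Destination key.
; Nothing in this Blueprint calls that relocation function.
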(event `self.ReceiveBeginPlay`
  (`GameplayStatics.PlaySound2D` "/Game/khi/Asset/Sound/SW_Day_Forest_Ambient_01.SW_Day_Forest_Ambient_01" 1.0 1.0 0.0 null null)
  (for _ (range (`self.Num Of Bird`))
    (bind _returnvalue (`|SpawnActorFromClass` "/Game/khi/Blueprint/BP_Bird.BP_Bird_C" (`self.GetTransform`) "AlwaysSpawn" "MultiplyWithRoot" null null))
    (`KismetArrayLibrary.Array_Add` (`self.Birds`) _returnvalue)))

(fn `RelocateBirdsAroundPlayer`
  (for _array_element (`self.Birds`)
    (`self.K2_SetActorLocation` _array_element (`/Game/khi/Blueprint/BP_Bird.GetRandomDest` _array_element) false false)
    (`BlackboardComponent.SetValueAsVector` (`AIBlueprintHelperLibrary.GetBlackboard` _array_element) "Destination" (`/Game/khi/Blueprint/BP_Bird.GetRandomDest` _array_element))))

(fn `UserConstructionScript`)