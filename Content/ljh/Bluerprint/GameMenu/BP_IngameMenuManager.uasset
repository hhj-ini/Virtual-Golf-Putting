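; In-world VR in-game menu manager actor with child BP_MenuButtons for exiting, height change and an unbound Mulligan.
; SetMenuState toggles button visibility and collision between the default menu and an exit confirmation that opens LV_Start_UI.
; The height button calls the game mode.
; After each player teleport, a delayed line trace repositions the menu on the surface behind or beside the player by handedness, turned toward them.
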(event `CheckbuttonPressed`
  (params (SelfButton :type "/Game/ljh/Bluerprint/StartMenu/BP_MenuButton Object Reference"))
  ; 2. Bind Events On Button Pressed
  (`GameplayStatics.OpenLevelBySoftObjectPtr` "/Game/ljh/Level/LV_Start_UI.LV_Start_UI"))

(event `MulliganButtonPressed`
  (params (SelfButton :type "/Game/ljh/Bluerprint/StartMenu/BP_MenuButton Object Reference"))
  ; 2. Bind Events On Button Pressed
)

(event `ExitButtonPressed`
  (params (SelfButton :type "/Game/ljh/Bluerprint/StartMenu/BP_MenuButton Object Reference"))
  ; 2. Bind Events On Button Pressed
  (`self.SetMenuState` "NewEnumerator1"))

(event `HeightButtonPressed`
  (params (SelfButton :type "/Game/ljh/Bluerprint/StartMenu/BP_MenuButton Object Reference"))
  ; 2. Bind Events On Button Pressed
  (if (`/Game/Platform/Interaction/Button/ButtonComponent.ButtonState` (`/Game/ljh/Bluerprint/StartMenu/BP_MenuButton.ButtonComponent` SelfButton))
    (bind _asgm_base_ui (cast `/Game/ljh/Bluerprint/GM_Base_UI` (`GameplayStatics.GetGameMode`)))
    (`/Game/ljh/Bluerprint/GM_Base_UI.ChangedHeightInteger` _asgm_base_ui)))

(event `BackbuttonPressed`
  (params (SelfButton :type "/Game/ljh/Bluerprint/StartMenu/BP_MenuButton Object Reference"))
  ; 2. Bind Events On Button Pressed
  (`self.SetMenuState` "NewEnumerator0"))

(event `self.ReceiveBeginPlay`
  (`|ExecutionSequence`
    (:`then_0`
      ; 1. Set Button Refs & Set ButtonTextName
      (bind _output_get (set `self.Button_Check` (`self.CastChildToBPMenuButton` (`self.CAC Check`))))
      (`self.SetButtonText` _output_get "Sure Exit?")
      (bind _output_get_2 (set `self.Button_Back` (`self.CastChildToBPMenuButton` (`self.CAC Back`))))
      (`self.SetButtonText` _output_get_2 "Back")
      (bind _output_get_3 (set `self.Button_Exit` (`self.CastChildToBPMenuButton` (`self.CAC Exit`))))
      (`self.SetButtonText` _output_get_3 "Exit")
      (bind _output_get_4 (set `self.Button_Mulligan` (`self.CastChildToBPMenuButton` (`self.CAC Mulligan`))))
      (`self.SetButtonText` _output_get_4 "Mulligan")
      (bind _output_get_5 (set `self.Button_Height` (`self.CastChildToBPMenuButton` (`self.CAC Height`))))
      (`self.SetButtonText` _output_get_5 "Height"))
    (:`then_1`
      ; 2. Bind Events On Button Pressed
      (add `/Game/ljh/Bluerprint/StartMenu/BP_MenuButton.OnButtonPressed` (`self.Button_Check`) (delegate `CheckbuttonPressed`))
      (add `/Game/ljh/Bluerprint/StartMenu/BP_MenuButton.OnButtonPressed` (`self.Button_Back`) (delegate `BackbuttonPressed`))
      (add `/Game/ljh/Bluerprint/StartMenu/BP_MenuButton.OnButtonPressed` (`self.Button_Exit`) (delegate `ExitButtonPressed`))
      (add `/Game/ljh/Bluerprint/StartMenu/BP_MenuButton.OnButtonPressed` (`self.Button_Height`) (delegate `HeightButtonPressed`)))
    (:`then_2`
      ; 3. Set Menu State DefaultMenu
      (`self.SetMenuState` "NewEnumerator0"))
    (:`then_3`
      (`KismetSystemLibrary.Delay` 0.2)
      (bind _returnvalue (`GameplayStatics.GetActorOfClass` "/Game/hhz/class/BP_VRCharacter_UI_Child.BP_VRCharacter_UI_Child_C"))
      (`/Engine/EditorBlueprintResources/StandardMacros.IsValid` _returnvalue
        (:`Is Valid`
          (bind _output_get_6 (set `self.Player` _returnvalue))
          (add `/Game/ljh/Bluerprint/BP_VRCharacter_UI.OnCharacterTeleport` _output_get_6 (delegate `UpdateLocation`)))))))

(event `self.ReceiveTick`
  (params (DeltaSeconds :type "Float (single-precision)")))

(event `UpdateLocation`
  (bind _player (`self.Player`))
  (bind _asgm_base_ui (cast `/Game/ljh/Bluerprint/GM_Base_UI` (`GameplayStatics.GetGameMode`)))
  (`KismetSystemLibrary.Delay` 1.0)
  (bind _returnvalue (+ (`self.K2_GetActorLocation` _player) (* (`self.GetActorRightVector` _player) (`self.SideOffset`) (`KismetMathLibrary.SelectFloat` 1.0 -1.0 (`/Game/ljh/Bluerprint/GM_Base_UI.IsRightHanded?` _asgm_base_ui))) (* (`self.GetActorForwardVector` _player) (`self.BackOffset`))))
  (bind (_outhit _returnvalue_2) (`KismetSystemLibrary.LineTraceSingle` (+ _returnvalue (0.0 0.0 500.0)) (+ _returnvalue (0.0 0.0 -1000.0)) "TraceTypeQuery1" false (`|MakeArray` (`self.Player`) :!type "Actor Object Reference")))
  (if _returnvalue_2
    (`self.K2_SetActorLocation` (`.Location` (`GameplayStatics.BreakHitResult` _outhit)))
    (`self.K2_SetActorRotation` (`KismetMathLibrary.MakeRotFromZX` (`.Normal` (`GameplayStatics.BreakHitResult` _outhit)) (`KismetMathLibrary.GetForwardVector` (`KismetMathLibrary.FindLookAtRotation` (`.Location` (`GameplayStatics.BreakHitResult` _outhit)) (`self.K2_GetActorLocation` (`self.Player`))))))))

(fn `CastChildToBPMenuButton`
  (params (InChildActorComponent :type "ChildActorComponent Object Reference"))
  (returns (OutBP_MenuActor :type "/Game/ljh/Bluerprint/StartMenu/BP_MenuButton Object Reference"))
  (bind _asbp_menu_button (cast `/Game/ljh/Bluerprint/StartMenu/BP_MenuButton` (`ChildActorComponent.ChildActor` InChildActorComponent))
    (:`then`
      _)
    (:`CastFailed`
      _))
  (return _asbp_menu_button))

(fn `GetTextOfButton`
  (params (InButton :type "/Game/ljh/Bluerprint/StartMenu/BP_MenuButton Object Reference"))
  (returns (OutButtonText :type Text))
  (bind _outbuttontext (`/Game/ljh/Bluerprint/StartMenu/BP_MenuButton.GetButtonText` InButton))
  (return _outbuttontext))

(fn `SetButtonText`
  (params (InBPMenuButton :type "/Game/ljh/Bluerprint/StartMenu/BP_MenuButton Object Reference") (InButtonNameText :type Text))
  (`TextRenderComponent.K2_SetText` (`/Game/ljh/Bluerprint/StartMenu/BP_MenuButton.ButtonText` InBPMenuButton) InButtonNameText)
  (return))

(fn `SetMenuState`
  (params (NewState :type "/Game/ljh/Bluerprint/GameMenu/E_IngameMenuState Enum" :default "NewEnumerator0"))
  (switch `/Game/ljh/Bluerprint/GameMenu/E_IngameMenuState` NewState
    (:`NewEnumerator0`
      ; State Change
      (`self.SetVisible & Collision` (`|MakeArray` (`self.Button_Check`)))
      (`self.SetVisible & Collision` (`|MakeArray` (`self.Button_Back`)))
      (`self.SetVisible & Collision` (`|MakeArray` (`self.Button_Exit`)) true)
      (`self.SetVisible & Collision` (`|MakeArray` (`self.Button_Mulligan`)) true)
      (`self.SetVisible & Collision` (`|MakeArray` (`self.Button_Height`)) true))
    (:`NewEnumerator1`
      (`self.SetVisible & Collision` (`|MakeArray` (`self.Button_Check`)) true)
      (`self.SetVisible & Collision` (`|MakeArray` (`self.Button_Back`)) true)
      (`self.SetVisible & Collision` (`|MakeArray` (`self.Button_Exit`)))
      (`self.SetVisible & Collision` (`|MakeArray` (`self.Button_Mulligan`)))
      (`self.SetVisible & Collision` (`|MakeArray` (`self.Button_Height`))))))

(fn `SetVisible & Collision`
  (params (InButtons :type "Array of /Game/ljh/Bluerprint/StartMenu/BP_MenuButton Object Reference") (activate :type Boolean))
  (if activate
    (for _array_element InButtons
      (`self.SetActorHiddenInGame` _array_element false)
      (`PrimitiveComponent.SetCollisionEnabled` (`/Game/ljh/Bluerprint/StartMenu/BP_MenuButton.ButtonComponent` _array_element) "QueryAndPhysics"))
    (else
      (for _array_element_2 InButtons
        (`self.SetActorHiddenInGame` _array_element_2 true)
        (`PrimitiveComponent.SetCollisionEnabled` (`/Game/ljh/Bluerprint/StartMenu/BP_MenuButton.ButtonComponent` _array_element_2) "NoCollision")))))

(fn `UserConstructionScript`)