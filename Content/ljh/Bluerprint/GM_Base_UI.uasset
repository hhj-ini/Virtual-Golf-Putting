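; GM_Base_UI is a game mode Blueprint for the golf game that holds handedness state and a height toggle.
; On BeginPlay it restores the saved right-handed flag from GI_Golf through ChangeHandMode, which writes it back to the game instance and calls the OnChangedHandMode dispatcher.
; ChangeInteger flips HeightInteger between 0 and 1.
; A handler bound to ChangedHeightInteger only prints a placeholder "Hello".
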(event `self.ReceiveBeginPlay`
  (bind _asgi_golf (cast `/Game/ljh/Level/GI_Golf` (`GameplayStatics.GetGameInstance`)))
  (bind _output_get (set `self.IsRightHanded?` (`/Game/ljh/Level/GI_Golf.SavedIsRightHanded` _asgi_golf)))
  (`self.ChangeHandMode` _output_get)
  (add `self.ChangedHeightInteger` (delegate `커스텀이벤트`)))

(event `커스텀이벤트`
  (`KismetSystemLibrary.PrintString` "Hello"))

(fn `ChangeHandMode`
  (params (NewMode :type Boolean))
  (bind _asgi_golf (cast `/Game/ljh/Level/GI_Golf` (`GameplayStatics.GetGameInstance`))
    (:`then`
      (set `/Game/ljh/Level/GI_Golf.SavedIsRightHanded` NewMode _asgi_golf))
    (:`CastFailed`
      _))
  (set `self.IsRightHanded?` NewMode)
  (`self.OnChangedHandMode`))

(fn `ChangeInteger`
  (if (`KismetMathLibrary.Conv_IntToBool` (`self.HeightInteger`))
    (set `self.HeightInteger` 0)
    (else
      (set `self.HeightInteger` 1))))

(fn `UserConstructionScript`
  (`parent.UserConstructionScript`))