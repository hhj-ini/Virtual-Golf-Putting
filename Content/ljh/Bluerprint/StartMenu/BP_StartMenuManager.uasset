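; Start menu manager that walks the player through ball difficulty, hand selection and Start, then server-travels to TestMap_UIVer.
; BeginPlay labels child-actor BP_MenuButtons, binds press events and opens the ball step.
; SetMenuState shows one button group at a time by toggling visibility and collision; Back steps backwards.
; Hand choice goes to GM_Base_UI via button-text comparison, while difficulty buttons only advance the menu.
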(event `StartbuttonPressed`
  (params (SelfButton :type "/Game/ljh/Bluerprint/StartMenu/BP_MenuButton Object Reference"))
  ; 2. Bind Events On Button Pressed
  (`self.SetMenuState` "NewEnumerator3")
  (`KismetSystemLibrary.ExecuteConsoleCommand` "ServerTravel TestMap_UIVer" null))

(event `BackButtonPressed`
  (params (SelfButton :type "/Game/ljh/Bluerprint/StartMenu/BP_MenuButton Object Reference"))
  ; 2. Bind Events On Button Pressed
  (if (`/Game/Platform/Interaction/Button/ButtonComponent.ButtonState` (`/Game/ljh/Bluerprint/StartMenu/BP_MenuButton.ButtonComponent` SelfButton))
    (switch `/Game/ljh/Bluerprint/StartMenu/E_StartMenuState` (`self.CurrentState`)
      (:`NewEnumerator0`
        (`self.SetMenuState` "NewEnumerator2"))
      (:`NewEnumerator2`
        (`self.SetMenuState` "NewEnumerator1")))))

(event `self.ReceiveBeginPlay`
  (bind _outbp_menuactor (`self.CastChildToBPMenuButton` (`self.NormalBallButton`)))
  (bind _outbp_menuactor_2 (`self.CastChildToBPMenuButton` (`self.RightButton`)))
  (bind _outbp_menuactor_3 (`self.CastChildToBPMenuButton` (`self.LeftButton`)))
  (bind _outbp_menuactor_4 (`self.CastChildToBPMenuButton` (`self.SlowBallButton`)))
  (bind _outbp_menuactor_5 (`self.CastChildToBPMenuButton` (`self.FastBallButton`)))
  (bind _outbp_menuactor_6 (`self.CastChildToBPMenuButton` (`self.BackButton`)))
  (`|ExecutionSequence`
    (:`then_0`
      ; 1. Set Button Refs & Set ButtonTextName
      (bind _output_get (set `self.Button_Start` (`self.CastChildToBPMenuButton` (`self.StartButton`))))
      (`self.SetButtonText` _output_get "Start")
      (`|ExecutionSequence`
        (:`then_0`
          (`self.SetButtonText` _outbp_menuactor_4 "Easy"))
        (:`then_1`
          (`self.SetButtonText` _outbp_menuactor_5 "Hard"))
        (:`then_2`
          (`self.SetButtonText` _outbp_menuactor "Normal"))
        (:`then_3`
          (set `self.Buttons_Spin` (`|MakeArray` _outbp_menuactor_4 _outbp_menuactor_5 _outbp_menuactor))
          (`|ExecutionSequence`
            (:`then_0`
              (`self.SetButtonText` _outbp_menuactor_3 "Left"))
            (:`then_1`
              (`self.SetButtonText` _outbp_menuactor_2 "Right"))
            (:`then_2`
              (set `self.Buttons_Hand` (`|MakeArray` _outbp_menuactor_3 _outbp_menuactor_2))
              (set `self.Button_Back` _outbp_menuactor_6)
              (`self.SetButtonText` _outbp_menuactor_6 "Back"))))))
    (:`then_1`
      ; 2. Bind Events On Button Pressed
      (add `/Game/ljh/Bluerprint/StartMenu/BP_MenuButton.OnButtonPressed` (`self.Button_Start`) (delegate `StartbuttonPressed`))
      (for _array_element (`self.Buttons_Spin`)
        (add `/Game/ljh/Bluerprint/StartMenu/BP_MenuButton.OnButtonPressed` _array_element (delegate `BallbuttonPressed`)))
      (for _array_element_2 (`self.Buttons_Hand`)
        (add `/Game/ljh/Bluerprint/StartMenu/BP_MenuButton.OnButtonPressed` _array_element_2 (delegate `HandbuttonPressed`))
        (add `/Game/ljh/Bluerprint/StartMenu/BP_MenuButton.OnButtonPressed` (`self.Button_Back`) (delegate `BackButtonPressed`))))
    (:`then_2`
      ; 3. Set Menu State Ball
      (`self.SetMenuState` "NewEnumerator1"))))

(event `HandbuttonPressed`
  (params (SelfButton :type "/Game/ljh/Bluerprint/StartMenu/BP_MenuButton Object Reference"))
  ; 2. Bind Events On Button Pressed
  (`|ExecutionSequence`
    (:`then_0`
      (bind _asgm_base_ui (cast `/Game/ljh/Bluerprint/GM_Base_UI` (`GameplayStatics.GetGameMode`)))
      (`/Game/ljh/Bluerprint/GM_Base_UI.ChangeHandMode` _asgm_base_ui (== (`self.GetTextOfButton` SelfButton) (`self.GetTextOfButton` (`self.CastChildToBPMenuButton` (`self.RightButton`))))))
    (:`then_1`
      (`self.SetMenuState` "NewEnumerator0"))))

(event `BallbuttonPressed`
  (params (SelfButton :type "/Game/ljh/Bluerprint/StartMenu/BP_MenuButton Object Reference"))
  ; 2. Bind Events On Button Pressed
  (`|ExecutionSequence`
    (:`then_1`
      (`self.SetMenuState` "NewEnumerator2"))))

(event `self.ReceiveTick`
  (params (DeltaSeconds :type "Float (single-precision)")))

(fn `CastChildToBPMenuButton`
  (params (InChildActorComponent :type "ChildActorComponent Object Reference"))
  (returns (OutBP_MenuActor :type "/Game/ljh/Bluerprint/StartMenu/BP_MenuButton Object Reference"))
  (bind _asbp_menu_button (cast `/Game/ljh/Bluerprint/StartMenu/BP_MenuButton` (`ChildActorComponent.ChildActor` InChildActorComponent))
    (:`then`
      _)
    (:`CastFailed`
      _))
  (return _asbp_menu_button))

(fn `Compare text of buttons`
  (params (`In CAC` :type "ChildActorComponent Object Reference") (`In Button` :type "/Game/ljh/Bluerprint/StartMenu/BP_MenuButton Object Reference"))
  (returns (`IsButtonTextEqual?` :type Boolean))
  (return (== (`self.GetTextOfButton` `In Button`) (`self.GetTextOfButton` (`self.CastChildToBPMenuButton` `In CAC`)))))

(fn `GetTextOfButton`
  (params (InButton :type "/Game/ljh/Bluerprint/StartMenu/BP_MenuButton Object Reference"))
  (returns (OutButtonText :type Text))
  (bind _outbuttontext (`/Game/ljh/Bluerprint/StartMenu/BP_MenuButton.GetButtonText` InButton))
  (return _outbuttontext))

(fn `SetButtonText`
  (params (InBPMenuButton :type "/Game/ljh/Bluerprint/StartMenu/BP_MenuButton Object Reference") (InButtonNameText :type Text))
  (`TextRenderComponent.K2_SetText` (`/Game/ljh/Bluerprint/StartMenu/BP_MenuButton.ButtonText` InBPMenuButton) InButtonNameText)
  (return))

(fn `SetMenuState`
  (params (NewState :type "/Game/ljh/Bluerprint/StartMenu/E_StartMenuState Enum" :default "NewEnumerator0"))
  (switch `/Game/ljh/Bluerprint/StartMenu/E_StartMenuState` NewState
    (:`NewEnumerator0`
      ; State Change
      (`self.SetVisible & Collision` (`|MakeArray` (`self.Button_Start`)) true)
      (`self.SetVisible & Collision` (`self.Buttons_Spin`))
      (`self.SetVisible & Collision` (`self.Buttons_Hand`))
      (set `self.CurrentState` "NewEnumerator0"))
    (:`NewEnumerator1`
      (`self.SetVisible & Collision` (`|MakeArray` (`self.Button_Start`)))
      (`self.SetVisible & Collision` (`self.Buttons_Spin`) true)
      (`self.SetVisible & Collision` (`self.Buttons_Hand`))
      (set `self.CurrentState` "NewEnumerator1"))
    (:`NewEnumerator2`
      (`self.SetVisible & Collision` (`|MakeArray` (`self.Button_Start`)))
      (`self.SetVisible & Collision` (`self.Buttons_Spin`))
      (`self.SetVisible & Collision` (`self.Buttons_Hand`) true)
      (set `self.CurrentState` "NewEnumerator2"))
    (:`NewEnumerator3`
      (`self.SetVisible & Collision` (`|MakeArray` (`self.Button_Start`)))
      (`self.SetVisible & Collision` (`self.Buttons_Spin`))
      (`self.SetVisible & Collision` (`self.Buttons_Hand`))
      (set `self.CurrentState` "NewEnumerator3"))))

(fn `SetVisible & Collision`
  (params (InButtons :type "Array of /Game/ljh/Bluerprint/StartMenu/BP_MenuButton Object Reference") (activate :type Boolean))
  (if activate
    (for _array_element InButtons
      (`self.SetActorHiddenInGame` _array_element false)
      (`PrimitiveComponent.SetCollisionEnabled` (`/Game/ljh/Bluerprint/StartMenu/BP_MenuButton.ButtonComponent` _array_element) "QueryAndPhysics"))
    (else
      (for _array_element_2 InButtons
        (`self.SetActorHiddenInGame` _array_element_2 true)
        (`PrimitiveComponent.SetCollisionEnabled` (`/Game/ljh/Bluerprint/StartMenu/BP_MenuButton.ButtonComponent` _array_element_2) "NoCollision")))))

(fn `UserConstructionScript`)