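; BP_BalckBall is a physics-simulated ball that detects when it stops moving and plays putting sounds on impact.
; BeginPlay enables physics, builds an array of two sounds and applies an initial force along X.
; Tick switches State between Default and Moving from the sphere's velocity, calling OnMoveEnd when it comes to rest.
; Hits outside the Moving state play a random sound at the ball; hits while moving only print a debug message.
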(event `self.ReceiveBeginPlay`
  (`PrimitiveComponent.SetSimulatePhysics` (`self.Sphere`) true)
  (bind _returnvalue (`GameplayStatics.CreateSound2D` "/Game/hhz/asset/PuttingSound.PuttingSound" 1.0 1.0 0.0 null))
  (bind _returnvalue_2 (`GameplayStatics.CreateSound2D` "/Game/hhz/asset/PuttingSound2.PuttingSound2" 1.0 1.0 0.0 null))
  (bind _output_get (set `self.SoundArray` (`|MakeArray` _returnvalue _returnvalue_2)))
  (`KismetSystemLibrary.PrintString` (`KismetStringLibrary.Conv_IntToString` (`KismetArrayLibrary.Array_Length` _output_get)))
  (`PrimitiveComponent.AddForce` (`self.Sphere`) (500.0 0.0 0.0) "None" false))

(event `self.ReceiveTick`
  (params (DeltaSeconds :type "Float (single-precision)"))
  (bind _returnvalue (`PrimitiveComponent.GetPhysicsLinearVelocity` (`self.Sphere`) "None"))
  (if (`KismetMathLibrary.Vector_IsNearlyZero` _returnvalue 0.001)
    (switch `/Game/hhz/class/E_BallState` (`self.State`)
      (:`NewEnumerator1`
        (set `self.State` "NewEnumerator0")
        (`self.OnMoveEnd`)))
    (else
      (switch `/Game/hhz/class/E_BallState` (`self.State`)
        (:`NewEnumerator0`
          (set `self.State` "NewEnumerator1"))))))

(event `self.Sphere.OnComponentHit`
  (params (HitComponent :type "PrimitiveComponent Object Reference") (OtherActor :type "Actor Object Reference") (OtherComp :type "PrimitiveComponent Object Reference") (NormalImpulse :type "Vector Structure") (Hit :type "HitResult Structure (by ref)"))
  (switch `/Game/hhz/class/E_BallState` (`self.State`)
    (:`NewEnumerator0`
      (`KismetSystemLibrary.PrintString` "hit")
      (cast `/Game/Platform/Core/Character/BP_VRCharacter` OtherActor
        (:`then`
          _)
        (:`CastFailed`
          _))
      (`GameplayStatics.PlaySoundAtLocation` (`AudioComponent.Sound` (`KismetArrayLibrary.Array_Random` (`self.SoundArray`))) (`SceneComponent.K2_GetComponentLocation` (`self.Sphere`)) (struct) 1.0 1.0 0.0 null null null null))
    (:`NewEnumerator1`
      (`KismetSystemLibrary.PrintString` "moving hit"))))

(fn `UserConstructionScript`)