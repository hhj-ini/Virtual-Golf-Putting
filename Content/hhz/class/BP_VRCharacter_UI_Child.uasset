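; Child VR character for a golf game that adds next-level teleporting and golf ball spawning.
; TeleportToNextLevel stops movement, issues camera fades around a VRMovementReference teleport and uses IsTeleporting as a re-entry guard.
; SpawnGolfBall line-traces vertically just ahead of the player to place the ball on the hit point.
; GI_Golf's BallState selects the white, black or red ball class, then BindTPEvent is called.
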(fn `SpawnGolfBall`
  (bind (_returnvalue_location _returnvalue_rotation) (`KismetMathLibrary.BreakTransform` (`self.GetTransform`)))
  (bind (_returnvalue_x _returnvalue_y _returnvalue_z) (`KismetMathLibrary.BreakVector` (+ _returnvalue_location (* (`self.GetActorForwardVector`) 50.0))))
  (bind _asgi_golf (cast `/Game/ljh/Level/GI_Golf` (`GameplayStatics.GetGameInstance`)))
  (bind _outhit (`KismetSystemLibrary.LineTraceSingle` (`KismetMathLibrary.MakeVector` _returnvalue_x _returnvalue_y (+ _returnvalue_z 100000.0)) (`KismetMathLibrary.MakeVector` _returnvalue_x _returnvalue_y (+ _returnvalue_z -100000.0)) "TraceTypeQuery4" true))
  (switch `/Game/ljh/Bluerprint/StartMenu/E_BallState` (`/Game/ljh/Level/GI_Golf.BallState` _asgi_golf)
    (:`NewEnumerator0`
      (bind _returnvalue (`KismetMathLibrary.MakeTransform` (+ (`.Location` (`GameplayStatics.BreakHitResult` _outhit)) (0.0 0.0 0.42)) _returnvalue_rotation))
      (`|SpawnActorFromClass` "/Game/hhz/class/BP_WhiteBall.BP_WhiteBall_C" _returnvalue "AdjustIfPossibleButAlwaysSpawn" "MultiplyWithRoot" null null))
    (:`NewEnumerator1`
      (`|SpawnActorFromClass` "/Game/hhz/class/BP_BalckBall.BP_BalckBall_C" _returnvalue "AdjustIfPossibleButAlwaysSpawn" "MultiplyWithRoot" null null))
    (:`NewEnumerator2`
      (`|SpawnActorFromClass` "/Game/hhz/class/BP_RedBall.BP_RedBall_C" _returnvalue "AdjustIfPossibleButAlwaysSpawn" "MultiplyWithRoot" null null)))
  (`self.BindTPEvent`))

(fn `TeleportToNextLevel`
  (params (Location :type "Vector Structure") (Rotation :type "Rotator Structure"))
  (if (not (`self.IsTeleporting`))
    (switch `/Game/Platform/Core/Character/MovementMode` "NewEnumerator0"
      (:`NewEnumerator0`
        (`MovementComponent.StopMovementImmediately` (`self.VRMovementReference`))
        (set `self.IsTeleporting` true)
        (`PlayerCameraManager.StartCameraFade` (`GameplayStatics.GetPlayerCameraManager` 0) 0.0 1.0 (`self.FadeOutDuration`) (`self.TeleportFadeColor`) false true)
        (bind (_outrotation _outnewposition) (`self.GetCharacterRotatedPosition` Location Rotation))
        (`VRBaseCharacterMovementComponent.PerformMoveAction_Teleport` (`self.VRMovementReference`) _outnewposition _outrotation "VRMOVEACTION_Velocity_None" false)
        (`PlayerCameraManager.StartCameraFade` (`GameplayStatics.GetPlayerCameraManager` 0) 1.0 0.0 (`self.FadeInDuration`) (`self.TeleportFadeColor`) false false)
        (set `self.IsTeleporting` false)))))

(fn `UserConstructionScript`
  (`parent.UserConstructionScript`))