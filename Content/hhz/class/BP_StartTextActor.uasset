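; BP_StartTextActor is an intro title actor that animates three text components, TextVirtual, TextSimulator and TextGolf, along Z when play begins.
; Each has its own timeline, whose ZLocation value is added to the component's current relative Z on every update, so movement accumulates.
; The next timeline is triggered from the previous one's Update through a short Delay, producing a staggered sequence rather than waiting for each to finish.
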(event `self.ReceiveBeginPlay`
  (bind _text_virtual (`self.Text_Virtual`))
  (bind _text_golf (`self.Text_Golf`))
  (bind _text_simulator (`self.Text_Simulator`))
  (bind (_relativelocation_x _relativelocation_y _relativelocation_z) (`KismetMathLibrary.BreakVector` (`SceneComponent.RelativeLocation` _text_virtual)))
  (bind (_relativelocation_x_2 _relativelocation_y_2 _relativelocation_z_2) (`KismetMathLibrary.BreakVector` (`SceneComponent.RelativeLocation` _text_golf)))
  (bind (_relativelocation_x_3 _relativelocation_y_3 _relativelocation_z_3) (`KismetMathLibrary.BreakVector` (`SceneComponent.RelativeLocation` _text_simulator)))
  (bind (_direction _zlocation) (`Timeline|TextVirtualTimeline`)
    (:`Update`
      (`SceneComponent.K2_SetRelativeLocation` _text_virtual (`KismetMathLibrary.MakeVector` _relativelocation_x _relativelocation_y (+ _relativelocation_z _zlocation)) false false)
      (`KismetSystemLibrary.Delay` 0.7)
      (bind (_direction_2 _zlocation_2) (`Timeline|TextSimulTimeline`)
        (:`Update`
          (`SceneComponent.K2_SetRelativeLocation` _text_simulator (`KismetMathLibrary.MakeVector` _relativelocation_x_3 _relativelocation_y_3 (+ _relativelocation_z_3 _zlocation_2)) false false)
          (`KismetSystemLibrary.Delay` 0.5)
          (bind (_direction_3 _zlocation_3) (`Timeline|TextGolfTimeline`)
            (:`Update`
              (`SceneComponent.K2_SetRelativeLocation` _text_golf (`KismetMathLibrary.MakeVector` _relativelocation_x_2 _relativelocation_y_2 (+ _relativelocation_z_2 _zlocation_3)) false false))))))))

(event `self.ReceiveTick`
  (params (DeltaSeconds :type "Float (single-precision)")))

(fn `UserConstructionScript`)